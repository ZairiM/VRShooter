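; BP_Target is a VR enemy target that launches upward as a randomly shaped figure and sometimes shoots at the player.
; On BeginPlay it picks a mesh from FiguresArray, randomizes its rotation and uniform scale, and applies a random upward velocity impulse.
; One in four targets waits a second, then spawns a BP_TargetBullet aimed at the Sphere component of the BP_PlayerVR pawn.
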(event `self.ReceiveBeginPlay`
  (bind _returnvalue (`SceneComponent.K2_GetComponentLocation` (`self.StaticMesh`)))
  (`StaticMeshComponent.SetStaticMesh` (`self.StaticMesh`) (`self.GetStaticMeshByFigure`))
  (`SceneComponent.K2_SetRelativeTransform` (`self.StaticMesh`) (`self.SetStaticMeshTransform`) false false)
  (`PrimitiveComponent.AddImpulse` (`self.StaticMesh`) (`KismetMathLibrary.MakeVector` 0.0 0.0 (`KismetMathLibrary.RandomFloatInRange` 700.0 1100.0)) "None" true)
  (bind _asbp_player_vr (cast `/Game/Blueprints/BP_PlayerVR` (`Controller.K2_GetPawn` (`GameplayStatics.GetPlayerController` 0))))
  (set `self.PlayerSphereReference` (`/Game/Blueprints/BP_PlayerVR.Sphere` _asbp_player_vr))
  ;[1 1 1] Solo una figura dispara de cada 4
  (switch `int` (`KismetMathLibrary.RandomIntegerInRange` 0 3)
    (:`0`
      (`KismetSystemLibrary.Delay` 1.0)
      (`|SpawnActorFromClass` "/Game/Blueprints/Enemies/BP_TargetBullet.BP_TargetBullet_C" (`KismetMathLibrary.MakeTransform` _returnvalue (`KismetMathLibrary.FindLookAtRotation` _returnvalue (`SceneComponent.K2_GetComponentLocation` (`self.PlayerSphereReference`))) (2.0 2.0 2.0)) "AdjustIfPossibleButAlwaysSpawn" "OverrideRootScale" null null))))

(fn `GetStaticMeshByFigure`
  (returns (ReturnValue :type "StaticMesh Object Reference"))
  (bind _figuresarray (`self.FiguresArray`))
  (return (`|GetArrayItem` _figuresarray (`KismetMathLibrary.RandomIntegerInRange` 0 (- (`KismetArrayLibrary.Array_Length` _figuresarray) 1)))))

(fn `SetStaticMeshTransform`
  (returns (ReturnValue :type "Transform Structure"))
  (return (`KismetMathLibrary.MakeTransform` (`SceneComponent.RelativeLocation` (`self.StaticMesh`)) (`KismetMathLibrary.RandomRotator` true) (`KismetMathLibrary.Conv_DoubleToVector` (`KismetMathLibrary.RandomFloatInRange` 0.5 1.5)))))

(fn `UserConstructionScript`)