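; BP_TargetBullet is an enemy projectile that damages the VR player on contact.
; When its Sphere begins overlapping a BP_PlayerVR, it stores the player reference and decrements that player's Health.
; It then spawns an impact vibration force feedback effect at both motion controllers and destroys itself.
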(event `self.Sphere.OnComponentBeginOverlap`
  (params (OverlappedComponent :type "PrimitiveComponent Object Reference") (OtherActor :type "Actor Object Reference") (OtherComp :type "PrimitiveComponent Object Reference") (OtherBodyIndex :type Integer) (bFromSweep :type Boolean) (SweepResult :type "HitResult Structure (by ref)"))
  (bind _playerreference (`self.PlayerReference`))
  (bind _asbp_player_vr (cast `/Game/Blueprints/BP_PlayerVR` OtherActor))
  (bind _output_get (set `self.PlayerReference` _asbp_player_vr))
  (`/Engine/EditorBlueprintResources/StandardMacros.DecrementInt` (`/Game/Blueprints/BP_PlayerVR.Health` _output_get)
    (:`  `
      (`GameplayStatics.SpawnForceFeedbackAtLocation` "/Game/Blueprints/FFE_ImpactVibration.FFE_ImpactVibration" (`SceneComponent.K2_GetComponentLocation` (`/Game/Blueprints/BP_PlayerVR.MotionControllerL` _playerreference)) (struct) false 1.0 0.0 null)
      (`GameplayStatics.SpawnForceFeedbackAtLocation` "/Game/Blueprints/FFE_ImpactVibration.FFE_ImpactVibration" (`SceneComponent.K2_GetComponentLocation` (`/Game/Blueprints/BP_PlayerVR.MotionControllerR` _playerreference)) (struct) false 1.0 0.0 null)
      (`self.K2_DestroyActor`))))

(fn `UserConstructionScript`)